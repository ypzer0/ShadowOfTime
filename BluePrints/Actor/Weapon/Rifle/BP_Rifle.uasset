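; Rifle weapon Blueprint that overrides no lifecycle logic and implements a Fire function for shooting.
; Fire calls CreateFireLine with camera location, direction and aim state to find the hit point, or the trace end on a miss.
; It spawns a rifle ammo actor at the muzzle socket rotated toward that point, so shots converge on the camera's target.
; Gunshot sound, muzzle flash and shell ejection effects accompany each shot.
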(fn `Fire`
  (params (CameraLocation :type "Vector Structure") (CameraForwardV :type "Vector Structure") (IsAim :type Boolean))
  (locals (LIsAim :type Boolean :default false) (LTargetLocation :type "Vector Structure"))
  (bind _skeletalmesh (`self.SkeletalMesh`))
  (bind _returnvalue (`SceneComponent.GetSocketLocation` (`self.SkeletalMesh`) (`.MuzzleSocketName_19_737B465E449B2D2C994C4EB21BBAE0EB` (break `/Game/ShadowOfTime/Structure/S_Weapon` (`self.Attributes`)))))
  (bind (_outhit _ishit) (`self.CreateFireLine` CameraLocation CameraForwardV IsAim))
  (if _ishit
    (bind (_bblockinghit _binitialoverlap _time _distance _location _impactpoint _normal _impactnormal _physmat _hitactor _hitcomponent _hitbonename _hititem _faceindex _tracestart _traceend) (`GameplayStatics.BreakHitResult` _outhit))
    (set `local.LTargetLocation` _location)
    (else
      (set `local.LTargetLocation` _traceend)))
  (`|SpawnActorFromClass` "/Game/ShadowOfTime/BluePrints/Actor/Weapon/Rifle/Actor_RifleAmmo.Actor_RifleAmmo_C" (`KismetMathLibrary.MakeTransform` _returnvalue (`KismetMathLibrary.FindLookAtRotation` _returnvalue (`local.LTargetLocation`))) "Undefined" "OverrideRootScale" self null)
  (`GameplayStatics.SpawnSoundAtLocation` "/Game/ShadowOfTime/BluePrints/Actor/Weapon/Rifle/Sounds/Rifle3.Rifle3" _returnvalue (struct) 1.0 1.0 0.0 null null)
  (`GameplayStatics.SpawnEmitterAttached` "/Game/ShadowOfTime/BluePrints/Ash/Particles/P_Rifle_Muzzleflash.P_Rifle_Muzzleflash" _skeletalmesh "MuzzleSocket")
  (`GameplayStatics.SpawnEmitterAttached` "/Game/ShadowOfTime/BluePrints/Ash/Particles/P_Rifle_ShellEject.P_Rifle_ShellEject" _skeletalmesh "ShellEjectionSocket"))

(fn `UserConstructionScript`
  (`parent.UserConstructionScript`))