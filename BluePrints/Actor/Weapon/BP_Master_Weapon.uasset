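; Master weapon Blueprint base with an empty Fire function and a shared hit-detection trace for its weapons.
; CreateFireLine runs a Visibility line trace over the weapon's attack distance and returns the hit result.
; When aiming, the trace runs from the camera along its forward vector; otherwise it runs from the mesh's muzzle socket along that socket's forward direction.
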(fn `CreateFireLine`
  (params (CameraLocation :type "Vector Structure") (CameraForwardV :type "Vector Structure") (IsAim :type Boolean))
  (returns (OutHit :type "HitResult Structure") (IsHit :type Boolean))
  (locals (LCameraLocation :type "Vector Structure") (LCameraForwardV :type "Vector Structure") (LIsAim :type Boolean))
  (bind _returnvalue (`SceneComponent.GetSocketLocation` (`self.SkeletalMesh`) (`.MuzzleSocketName_19_737B465E449B2D2C994C4EB21BBAE0EB` (break `/Game/ShadowOfTime/Structure/S_Weapon` (`self.Attributes`)))))
  (set `local.LCameraLocation` CameraLocation)
  (set `local.LCameraForwardV` CameraForwardV)
  (set `local.LIsAim` IsAim)
  (bind (_outhit _returnvalue_2) (`KismetSystemLibrary.LineTraceSingle` (select `bool` (`local.LIsAim`) :`false` _returnvalue :`true` (`local.LCameraLocation`)) (select `bool` (`local.LIsAim`) :`false` (+ _returnvalue (* (`KismetMathLibrary.GetForwardVector` (`SceneComponent.GetSocketRotation` (`self.SkeletalMesh`) (`.MuzzleSocketName_19_737B465E449B2D2C994C4EB21BBAE0EB` (break `/Game/ShadowOfTime/Structure/S_Weapon` (`self.Attributes`))))) (`.AttackDistance_16_C8246FBF4642C0F28E3E65862D6AD82E` (break `/Game/ShadowOfTime/Structure/S_Weapon` (`self.Attributes`))))) :`true` (+ (`local.LCameraLocation`) (* (`local.LCameraForwardV`) (`.AttackDistance_16_C8246FBF4642C0F28E3E65862D6AD82E` (break `/Game/ShadowOfTime/Structure/S_Weapon` (`self.Attributes`)))))) "TraceTypeQuery1"))
  (return _outhit _returnvalue_2))

(fn `Fire`
  (params (CameraLocation :type "Vector Structure") (CameraForwardV :type "Vector Structure") (IsAim :type Boolean)))

(fn `UserConstructionScript`)